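; Behavior tree task that advances an enemy's patrol index after it reaches a path point.
; It steps CurrentPathIndex by PathDirection while the next index is valid in the BP_EnemyBase patrol path.
; At the path's end, PatrolPathBehavior decides: stay put, flip the direction to patrol back, or reset the index to zero to loop.
; Each of these branches finishes successfully.
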(event EventReceiveExecuteAI
  (params (OwnerController :type AI%20Controller%20Object%20Reference) (ControlledPawn :type Pawn%20Object%20Reference))
  (bind _asbp_enemy_base (Utilities|Casting|CastToBP_EnemyBase ControlledPawn))
  (bind _output_get (Variables|Default|SetEnemyPawn _asbp_enemy_base))
  (if (Utilities|Array|IsValidIndex (Variables|/Game/Blueprint/AI/BP_EnemyBase.BP_EnemyBase_C|GetPatrolPath _output_get) (+ (Variables|/Game/Blueprint/AI/BP_EnemyBase.BP_EnemyBase_C|GetCurrentPathIndex _output_get) (Variables|/Game/Blueprint/AI/BP_EnemyBase.BP_EnemyBase_C|GetPathDirection _output_get)))
    (Variables|/Game/Blueprint/AI/BP_EnemyBase.BP_EnemyBase_C|SetCurrentPathIndex (Variables|Default|GetEnemyPawn) (+ (Variables|/Game/Blueprint/AI/BP_EnemyBase.BP_EnemyBase_C|GetCurrentPathIndex (Variables|Default|GetEnemyPawn)) (Variables|/Game/Blueprint/AI/BP_EnemyBase.BP_EnemyBase_C|GetPathDirection (Variables|Default|GetEnemyPawn))))
    (AI|BehaviorTree|FinishExecute true)
    (else
      (switch Utilities|FlowControl|Switch|SwitchonEnum_PatrolPathEnding (Variables|/Game/Blueprint/AI/BP_EnemyBase.BP_EnemyBase_C|GetPatrolPathBehavior (Variables|Default|GetEnemyPawn))
        (:NewEnumerator0
          (AI|BehaviorTree|FinishExecute true))
        (:NewEnumerator1
          (Variables|/Game/Blueprint/AI/BP_EnemyBase.BP_EnemyBase_C|SetPathDirection (Variables|Default|GetEnemyPawn) (* (Variables|/Game/Blueprint/AI/BP_EnemyBase.BP_EnemyBase_C|GetPathDirection (Variables|Default|GetEnemyPawn)) -1))
          (AI|BehaviorTree|FinishExecute true))
        (:NewEnumerator2
          (Variables|/Game/Blueprint/AI/BP_EnemyBase.BP_EnemyBase_C|SetCurrentPathIndex (Variables|Default|GetEnemyPawn) 0)
          (AI|BehaviorTree|FinishExecute true))))))