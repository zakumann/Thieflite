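; Behavior tree task that picks the next patrol destination and wait time for a BP_EnemyBase pawn.
; It reads the patrol point at the pawn's current path index and writes a random reachable point near it to the target blackboard key.
; It also writes a wait time randomized around that point's wait time by its deviation, then finishes successfully without advancing the index.
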(event EventReceiveExecuteAI
  (params (OwnerController :type AI%20Controller%20Object%20Reference) (ControlledPawn :type Pawn%20Object%20Reference))
  (bind _asbp_enemy_base (Utilities|Casting|CastToBP_EnemyBase ControlledPawn))
  (bind _output_get (Variables|Default|SetEnemyPawn _asbp_enemy_base))
  (AI|BehaviorTree|SetBlackboardValueasVector (Variables|Default|GetBB_TargetVector) (.RandomLocation (AI|Navigation|GetRandomReachablePointinRadius (Transformation|GetActorLocation (Utilities|Array|Get(acopy) (Variables|/Game/Blueprint/AI/BP_EnemyBase.BP_EnemyBase_C|GetPatrolPath _output_get) (Variables|/Game/Blueprint/AI/BP_EnemyBase.BP_EnemyBase_C|GetCurrentPathIndex _output_get))) 2e+01 0 0)))
  (Class|BTFunctionLibrary|SetBlackboardValueasFloat (Variables|Default|GetBB_WaitTime) (Math|Random|RandomFloatinRange (- (Variables|/Game/Blueprint/AI/A_PathPoint.A_PathPoint_C|GetWaitTime (Utilities|Array|Get(acopy) (Variables|/Game/Blueprint/AI/BP_EnemyBase.BP_EnemyBase_C|GetPatrolPath (Variables|Default|GetEnemyPawn)) (Variables|/Game/Blueprint/AI/BP_EnemyBase.BP_EnemyBase_C|GetCurrentPathIndex (Variables|Default|GetEnemyPawn)))) (Variables|/Game/Blueprint/AI/A_PathPoint.A_PathPoint_C|GetWaitDeviation (Utilities|Array|Get(acopy) (Variables|/Game/Blueprint/AI/BP_EnemyBase.BP_EnemyBase_C|GetPatrolPath (Variables|Default|GetEnemyPawn)) (Variables|/Game/Blueprint/AI/BP_EnemyBase.BP_EnemyBase_C|GetCurrentPathIndex (Variables|Default|GetEnemyPawn))))) (+ (Variables|/Game/Blueprint/AI/A_PathPoint.A_PathPoint_C|GetWaitTime (Utilities|Array|Get(acopy) (Variables|/Game/Blueprint/AI/BP_EnemyBase.BP_EnemyBase_C|GetPatrolPath (Variables|Default|GetEnemyPawn)) (Variables|/Game/Blueprint/AI/BP_EnemyBase.BP_EnemyBase_C|GetCurrentPathIndex (Variables|Default|GetEnemyPawn)))) (Variables|/Game/Blueprint/AI/A_PathPoint.A_PathPoint_C|GetWaitDeviation (Utilities|Array|Get(acopy) (Variables|/Game/Blueprint/AI/BP_EnemyBase.BP_EnemyBase_C|GetPatrolPath (Variables|Default|GetEnemyPawn)) (Variables|/Game/Blueprint/AI/BP_EnemyBase.BP_EnemyBase_C|GetCurrentPathIndex (Variables|Default|GetEnemyPawn)))))))
  (AI|BehaviorTree|FinishExecute true))